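; BP_SwingingDoor is an activatable door that swings open once when activated.
; Activate sets IsOpen, which blocks repeat triggers, and starts a one-second countdown.
; While the countdown runs, Tick yaws the root component by RotationAmount per second, so that value approximates the total swing angle.
; The file has no closing logic, and the last frame can slightly overshoot because the step is not clamped.
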(event `self.Activate`
  (if (not (`self.isOpen`))
    (set `self.currentRotationTime` 1.0)
    (set `self.isOpen` true)))

(event `self.ReceiveTick`
  (params (DeltaSeconds :type "Float (single-precision)"))
  (if (> (`self.currentRotationTime`) 0.0)
    (`SceneComponent.K2_AddLocalRotation` (`self.DefaultSceneRoot`) (`KismetMathLibrary.MakeRotator` 0.0 0.0 (* DeltaSeconds (`self.RotationAmount`))) false false)
    (set `self.currentRotationTime` (- (`self.currentRotationTime`) DeltaSeconds))))

(fn `UserConstructionScript`
  (`parent.UserConstructionScript`))