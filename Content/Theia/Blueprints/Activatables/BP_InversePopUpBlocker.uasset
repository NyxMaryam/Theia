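; BP_InversePopUpBlocker is an activatable blocker whose Cube sinks when activated, the inverse of a pop-up.
; Activate instantly moves the Cube 30 units below its relative origin, and Reset returns it to that origin.
; An Activated flag guards both events against repeat calls, and neither move sweeps for collision.
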(event `self.Activate`
  (if (not (`self.Activated`))
    (set `self.Activated` true)
    (`SceneComponent.K2_SetRelativeLocation` (`self.Cube`) (0.0 0.0 -30.0) false false)))

(event `self.Reset`
  (if (`self.Activated`)
    (set `self.Activated` false)
    (`SceneComponent.K2_SetRelativeLocation` (`self.Cube`) (0.0 0.0 0.0) false false)))

(fn `UserConstructionScript`
  (`parent.UserConstructionScript`))