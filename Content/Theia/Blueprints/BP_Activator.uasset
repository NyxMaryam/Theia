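; BP_Activator is an activator Blueprint that shows its active or inactive state on a linked wire mesh.
; ToggleWire checks that WireMesh is valid, then swaps the first material on its static mesh component between the active and inactive wire materials.
; Reset and the construction script are empty, and nothing in this graph calls ToggleWire.
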(event `Reset`)

(fn `ToggleWire`
  (params (IsActive :type Boolean))
  (`/Engine/EditorBlueprintResources/StandardMacros.IsValid` (`self.WireMesh`)
    (:`Is Valid`
      (if true
        (if IsActive
          (`PrimitiveComponent.SetMaterial` (`self.GetComponentByClass` (`self.WireMesh`) "/Script/Engine.StaticMeshComponent") 0 (`self.ActiveWireMaterial`))
          (else
            (`PrimitiveComponent.SetMaterial` (`self.GetComponentByClass` (`self.WireMesh`) "/Script/Engine.StaticMeshComponent") 0 (`self.InactiveWireMaterial`))))))))

(fn `UserConstructionScript`)