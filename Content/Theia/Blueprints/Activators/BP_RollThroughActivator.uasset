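; BP_RollThroughActivator is an activator that fires when a BP_TheiaSphere overlaps it.
; The first such overlap calls Activate on each linked activatable, setting IsActivated and toggling the wire inside that loop, so an empty list leaves it unactivated.
; Reset clears the flag and toggles the wire off so it can fire again, without calling anything on the linked activatables.
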(event `self.ReceiveActorBeginOverlap`
  (params (OtherActor :type "Actor Object Reference"))
  (cast `/Game/Theia/Blueprints/BP_TheiaSphere` OtherActor)
  (if (not (`self.IsActivated`))
    (for _array_element (`self.LinkedActivatables`)
      (`/Game/Theia/Blueprints/BP_Activatable.Activate` _array_element)
      (bind _output_get (set `self.IsActivated` true))
      (`self.ToggleWire` _output_get))))

(event `self.Reset`
  (if (`self.IsActivated`)
    (bind _output_get (set `self.IsActivated` false))
    (`self.ToggleWire` _output_get)))

(fn `UserConstructionScript`
  (`parent.UserConstructionScript`))