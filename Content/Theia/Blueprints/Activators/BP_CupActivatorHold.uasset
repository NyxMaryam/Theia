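; BP_CupActivatorHold is a hold-style activator that keeps its linked activatables on only while an actor overlaps it.
; Begin overlap calls Activate on each entry in LinkedActivatables, and end overlap calls Reset on each, with IsActivated guarding against repeat triggers.
; The flag and ToggleWire update inside each loop, and overlaps are neither filtered nor counted, so any actor leaving resets an active activator.
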(event `self.ReceiveActorBeginOverlap`
  (params (OtherActor :type "Actor Object Reference"))
  (if (not (`self.IsActivated`))
    (for _array_element (`self.LinkedActivatables`)
      (`/Game/Theia/Blueprints/BP_Activatable.Activate` _array_element)
      (bind _output_get (set `self.IsActivated` true))
      (`self.ToggleWire` _output_get))))

(event `self.ReceiveActorEndOverlap`
  (params (OtherActor :type "Actor Object Reference"))
  (if (`self.IsActivated`)
    (for _array_element (`self.LinkedActivatables`)
      (`/Game/Theia/Blueprints/BP_Activatable.Reset` _array_element)
      (bind _output_get (set `self.IsActivated` false))
      (`self.ToggleWire` _output_get))))

(fn `UserConstructionScript`
  (`parent.UserConstructionScript`))